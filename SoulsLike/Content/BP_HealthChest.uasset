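; Health potion chest actor that opens once on Interact, playing the chest animation and printing a pickup message.
; After a delay it destroys the light and potion components and sets PotionFound.
; A trigger box sets NearChest on BP_Character as the player enters or leaves, and briefly shows an interact prompt on first entry only.
; The potion widget creation is unconnected, and no health is granted here.
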(event `self.ReceiveTick`
  (params (DeltaSeconds :type "Float (single-precision)")))

(event `self.Interact`
  (`KismetSystemLibrary.PrintString` (`KismetStringLibrary.Conv_BoolToString` (`self.potionFound`)) true true (struct :`R` 1.0 :`G` 0.593999 :`B` 0.055236 :`A` 1.0))
  (`/Engine/EditorBlueprintResources/StandardMacros.DoOnce` false
    (:`Completed`
      (`SkeletalMeshComponent.PlayAnimation` (`self.old_Chest`) "/Game/Models/old_Chest_Anim.old_Chest_Anim" false)
      (`KismetSystemLibrary.PrintString` "You got the potion")
      (`KismetSystemLibrary.Delay` 2.5)
      (`ActorComponent.K2_DestroyComponent` (`self.PointLight`))
      (`ActorComponent.K2_DestroyComponent` (`self.HealthPotion`))
      (set `self.potionFound` true))))

(event `self.ReceiveBeginPlay`
  ;[1 0.1705 0.9269] Text Prompt
  (bind _returnvalue (`|GenericCreateObject` "/Game/Interact_TextBP.Interact_TextBP_C"))
  (set `self.InteractPrompt` _returnvalue))

(event `self.Box.OnComponentBeginOverlap`
  (params (OverlappedComponent :type "PrimitiveComponent Object Reference") (OtherActor :type "Actor Object Reference") (OtherComp :type "PrimitiveComponent Object Reference") (OtherBodyIndex :type Integer) (bFromSweep :type Boolean) (SweepResult :type "HitResult Structure (by ref)"))
  (bind _interactprompt (`self.InteractPrompt`))
  ;[1 0.1705 0.9269] Text Prompt
  (if (== OtherActor (`GameplayStatics.GetPlayerCharacter` 0))
    (bind _asbp_character (cast `/Game/MyContent/BP_Character` (`GameplayStatics.GetPlayerCharacter` 0)))
    (set `/Game/MyContent/BP_Character.nearChest` true _asbp_character)
    (`/Engine/EditorBlueprintResources/StandardMacros.DoOnce` false
      (:`Completed`
        (`UserWidget.AddToViewport` _interactprompt 0)
        (`KismetSystemLibrary.Delay` 1.0)
        (`Widget.RemoveFromParent` _interactprompt :!label _label)))))

(event `self.Box.OnComponentEndOverlap`
  (params (OverlappedComponent :type "PrimitiveComponent Object Reference") (OtherActor :type "Actor Object Reference") (OtherComp :type "PrimitiveComponent Object Reference") (OtherBodyIndex :type Integer))
  ;[1 0.1705 0.9269] Text Prompt
  (if (== (`GameplayStatics.GetPlayerCharacter` 0) OtherActor)
    (bind _asbp_character (cast `/Game/MyContent/BP_Character` (`GameplayStatics.GetPlayerCharacter` 0)))
    (set `/Game/MyContent/BP_Character.nearChest` false _asbp_character)
    (goto _label)))

(fn `UserConstructionScript`)