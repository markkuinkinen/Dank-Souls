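; BP_Dummy is a damageable dummy character that reacts to hits and plays a death montage when its health runs out.
; AnyDamage passes through a DoOnce gate, subtracts from Health, then plays either the impact or death montage.
; The gate resets after a delay equal to the impact montage's length, so damage during that window is ignored.
; Death never resets the gate, so later damage has no effect.
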(event `self.ReceiveAnyDamage`
  (params (Damage :type "Float (single-precision)") (DamageType :type "DamageType Object Reference") (InstigatedBy :type "Controller Object Reference") (DamageCauser :type "Actor Object Reference"))
  (`/Engine/EditorBlueprintResources/StandardMacros.DoOnce` false :!label _label
    (:`Completed`
      (bind _output_get (set `self.Health` (- (`self.Health`) Damage)))
      (if (<= _output_get 0.0)
        (`self.PlayAnimMontage` "/Game/MyContent/OLD_character_Model/Animations/MONTAGE_Death.MONTAGE_Death")
        (else
          (bind _returnvalue (`self.PlayAnimMontage` "/Game/MyContent/OLD_character_Model/Animations/Montage_Impact.Montage_Impact"))
          (`KismetSystemLibrary.Delay` _returnvalue)
          (goto _label :!via `Reset`))))))

(event `/Game/MyContent/Interfaces_Events/Damage_Interface.ApplyDamage`)

(fn `UserConstructionScript`)