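; BP_Sword is a collectible sword pickup that shows an interaction prompt when the player enters its SwordBox.
; The prompt widget is created at BeginPlay and removed after a short delay or when the player leaves.
; Interact toggles visibility on both this sword and the BP_Character's sword, then flags the sword as collected and visible in BP_GameMode.
; Visibility is flipped rather than set, with no guard against repeat interaction.
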(event `/Game/MyContent/Interfaces_Events/Interact_Interface.Interact`
  (`SceneComponent.ToggleVisibility` (`self.Sword`) true)
  (bind _asbp_character (cast `/Game/MyContent/BP_Character` (`GameplayStatics.GetPlayerCharacter` 0)))
  (`SceneComponent.ToggleVisibility` (`/Game/MyContent/BP_Character.Sword` _asbp_character) false)
  (bind _asbp_game_mode (cast `/Game/MyContent/BP_GameMode` (`GameplayStatics.GetGameMode`)))
  (set `/Game/MyContent/BP_GameMode.SwordCollected` true _asbp_game_mode)
  (set `/Game/MyContent/BP_GameMode.sowrdVisible` true _asbp_game_mode))

(event `self.ReceiveBeginPlay`
  ;[1 1 1] Comment
  (bind _returnvalue (`|GenericCreateObject` "/Game/MyContent/UI/Interact_TextBP.Interact_TextBP_C"))
  (set `self.InteractPromt` _returnvalue))

(event `self.SwordBox.OnComponentBeginOverlap`
  (params (OverlappedComponent :type "PrimitiveComponent Object Reference") (OtherActor :type "Actor Object Reference") (OtherComp :type "PrimitiveComponent Object Reference") (OtherBodyIndex :type Integer) (bFromSweep :type Boolean) (SweepResult :type "HitResult Structure (by ref)"))
  (bind _interactpromt (`self.InteractPromt`))
  ;[1 1 1] Comment
  (if (== OtherActor (`GameplayStatics.GetPlayerCharacter` 0))
    (`UserWidget.AddToViewport` _interactpromt 0)
    (`KismetSystemLibrary.Delay` 1.0)
    (`Widget.RemoveFromParent` _interactpromt :!label _label)))

(event `self.SwordBox.OnComponentEndOverlap`
  (params (OverlappedComponent :type "PrimitiveComponent Object Reference") (OtherActor :type "Actor Object Reference") (OtherComp :type "PrimitiveComponent Object Reference") (OtherBodyIndex :type Integer))
  ;[1 1 1] Comment
  (if (== (`GameplayStatics.GetPlayerCharacter` 0) OtherActor)
    (goto _label)))

(fn `UserConstructionScript`)