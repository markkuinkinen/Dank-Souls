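; BP_Gate is a gate that opens once the player uses a found key.
; KeyInteract checks KeyFound on BP_GameMode, then sets KeyUsed, clears KeyFound and prints a debug message.
; Tick polls KeyUsed and, through a DoOnce, destroys the Closed and Box components and toggles Open's visibility.
; Key state lives on the game mode, so every gate instance reacts to the same KeyUsed flag.
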(event `self.ReceiveTick`
  (params (DeltaSeconds :type "Float (single-precision)"))
  (bind _asbp_game_mode (cast `/Game/MyContent/BP_GameMode` (`GameplayStatics.GetGameMode`)))
  (if (`/Game/MyContent/BP_GameMode.KeyUsed` _asbp_game_mode)
    (`/Engine/EditorBlueprintResources/StandardMacros.DoOnce` false
      (:`Completed`
        (`ActorComponent.K2_DestroyComponent` (`self.Closed`))
        (`SceneComponent.ToggleVisibility` (`self.Open`) false)
        (`ActorComponent.K2_DestroyComponent` (`self.Box`))))))

(event `/Game/MyContent/Interfaces_Events/Key_Inetrface.KeyInteract`
  (bind _asbp_game_mode (cast `/Game/MyContent/BP_GameMode` (`GameplayStatics.GetGameMode`)))
  (if (`/Game/MyContent/BP_GameMode.KeyFound` _asbp_game_mode)
    (set `/Game/MyContent/BP_GameMode.KeyUsed` true _asbp_game_mode)
    (`KismetSystemLibrary.PrintString` "Hello")
    (set `/Game/MyContent/BP_GameMode.KeyFound` false _asbp_game_mode)))

(fn `UserConstructionScript`)