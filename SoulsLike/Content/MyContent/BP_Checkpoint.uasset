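; BP_Checkpoint is a checkpoint that sets the player's respawn point and acts as a rest spot.
; Overlapping Box caches the character and GameMode, then stores the Pos component's transform as RespawnTransform.
; Interact uses those cached references to alternately start and stop a sitting montage, raising empty static health charges to one upon sitting.
; MessageCollision shows an interact prompt widget once, removing it after a short delay or when the player leaves.
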(event `/Game/MyContent/Interfaces_Events/Interact_Interface.Interact`
  (`/Engine/EditorBlueprintResources/StandardMacros.FlipFlop`
    (:`A`
      (`Character.PlayAnimMontage` (stale `self.Box.OnComponentBeginOverlap` _asbp_character) "/Game/MyContent/New_animations/Player_Sitting.Player_Sitting" 1.0 "None")
      (if (== (`/Game/MyContent/BP_GameMode.HealthChargesStatic` (stale `self.Box.OnComponentBeginOverlap` _asbp_game_mode)) 0)
        (set `/Game/MyContent/BP_GameMode.HealthChargesStatic` 1 (stale `self.Box.OnComponentBeginOverlap` _asbp_game_mode))))
    (:`B`
      (`Character.StopAnimMontage` (stale `self.Box.OnComponentBeginOverlap` _asbp_character) "/Game/MyContent/New_animations/Player_Sitting.Player_Sitting"))))

(event `self.Box.OnComponentBeginOverlap`
  (params (OverlappedComponent :type "PrimitiveComponent Object Reference") (OtherActor :type "Actor Object Reference") (OtherComp :type "PrimitiveComponent Object Reference") (OtherBodyIndex :type Integer) (bFromSweep :type Boolean) (SweepResult :type "HitResult Structure (by ref)"))
  (bind _asbp_character (cast `/Game/MyContent/BP_Character` OtherActor))
  (bind _asbp_game_mode (cast `/Game/MyContent/BP_GameMode` (`GameplayStatics.GetGameMode`)))
  (set `/Game/MyContent/BP_GameMode.Respawn Transform` (`SceneComponent.K2_GetComponentToWorld` (`self.Pos`)) _asbp_game_mode))

(event `self.ReceiveBeginPlay`
  ;[1 0.1705 0.9269] Text Prompt
  (bind _returnvalue (`|GenericCreateObject` "/Game/MyContent/UI/Interact_TextBP.Interact_TextBP_C"))
  (set `self.InteractPrompt` _returnvalue))

(event `self.MessageCollision.OnComponentBeginOverlap`
  (params (OverlappedComponent :type "PrimitiveComponent Object Reference") (OtherActor :type "Actor Object Reference") (OtherComp :type "PrimitiveComponent Object Reference") (OtherBodyIndex :type Integer) (bFromSweep :type Boolean) (SweepResult :type "HitResult Structure (by ref)"))
  (bind _interactprompt (`self.InteractPrompt`))
  ;[1 0.1705 0.9269] Text Prompt
  (if (== OtherActor (`GameplayStatics.GetPlayerCharacter` 0))
    (`/Engine/EditorBlueprintResources/StandardMacros.DoOnce` false
      (:`Completed`
        (`UserWidget.AddToViewport` _interactprompt 0)
        (`KismetSystemLibrary.Delay` 1.0)
        (`Widget.RemoveFromParent` _interactprompt :!label _label)))))

(event `self.MessageCollision.OnComponentEndOverlap`
  (params (OverlappedComponent :type "PrimitiveComponent Object Reference") (OtherActor :type "Actor Object Reference") (OtherComp :type "PrimitiveComponent Object Reference") (OtherBodyIndex :type Integer))
  ;[1 0.1705 0.9269] Text Prompt
  (if (== (`GameplayStatics.GetPlayerCharacter` 0) OtherActor)
    (goto _label)))

(fn `UserConstructionScript`)