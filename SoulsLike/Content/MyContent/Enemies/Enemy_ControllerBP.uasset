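; Enemy AI controller that runs the Enemy_BT behavior tree on BeginPlay and feeds it a target from AI perception.
; A successful sight stimulus stores the perceived actor in the "Target Actor" blackboard key.
; Losing sight, or receiving any non-sight stimulus, clears that key.
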(event `self.ReceiveBeginPlay`
  (`self.RunBehaviorTree` "/Game/MyContent/Enemies/Enemy_BT.Enemy_BT"))

(event `self.AIPerception.OnTargetPerceptionUpdated`
  (params (Actor :type "Actor Object Reference") (Stimulus :type "AIStimulus Structure"))
  ;[1 0.4663 0.8971] detect and chase target
  (bind _returnvalue (`AIPerceptionSystem.GetSenseClassForStimulus` Stimulus))
  (if (== _returnvalue "/Script/AIModule.AISense_Sight")
    (if (`.bSuccessfullySensed` (break `AIStimulus` Stimulus))
      (`BlackboardComponent.SetValueAsObject` (`AIBlueprintHelperLibrary.GetBlackboard` null) "Target Actor" Actor)
      (else
        (`BlackboardComponent.SetValueAsObject` (`AIBlueprintHelperLibrary.GetBlackboard` null) "Target Actor" null :!label _label)))
    (else
      (goto _label))))

(fn `UserConstructionScript`)