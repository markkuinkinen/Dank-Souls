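; Enemy character Blueprint that chases the player on sight and plays a melee attack montage on arrival.
; PawnSensing triggers FollowPlayer, which runs AI MoveTo toward the player, then plays the montage behind a CanAttack gate held for its duration.
; Tick clears the sight flag each frame, but its stop-movement branch never fires.
; The construction script snaps the weapon to the hand socket; wander and debug nodes are disconnected.
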(event `self.ReceiveBeginPlay`
  ;[1 0.2956 0.9014] ai follow
)

(event `self.PawnSensing.OnSeePawn`
  (params (Pawn :type "Pawn Object Reference"))
  ;[1 0.2956 0.9014] ai follow
  (set `self.isSeeingPlayer` true)
  (`self.FollowPlayer`))

(event `FollowPlayer`
  ;[1 0.2956 0.9014] ai follow
  (set `self.canAttack` true)
  (if (`self.isSeeingPlayer`)
    (`|AIMoveTo` self (0.0 0.0 0.0) (`GameplayStatics.GetPlayerCharacter` 0) 90.0
      (:`OnSuccess`
        (if (`self.canAttack`)
          (set `self.canAttack` false)
          (bind _returnvalue (`self.PlayAnimMontage` "/Game/MyContent/Enemies/anims/Attack_MOntage.Attack_MOntage"))
          (`KismetSystemLibrary.Delay` _returnvalue)
          (set `self.canAttack` true))))
    (else
      (set `self.isSeeingPlayer` false))))

(event `self.ReceiveTick`
  (params (DeltaSeconds :type "Float (single-precision)"))
  ;[1 0.2956 0.9014] ai follow
  (`|ExecutionSequence`
    (:`then_0`
      (set `self.isSeeingPlayer` false)
      (if (not true)
        (`MovementComponent.StopMovementImmediately` (`self.CharacterMovement`))))))

(fn `UserConstructionScript`
  (`SceneComponent.K2_AttachToComponent` (`self.weapon`) (`self.Mesh`) "hand_rSocket" "SnapToTarget" "SnapToTarget" "KeepRelative" true))