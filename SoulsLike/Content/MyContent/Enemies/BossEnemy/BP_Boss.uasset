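; BP_Boss is a boss enemy that performs a ranged fire attack while the player character is alive.
; Attack plays the ranged-attack montage, using an IsAttacking flag to block re-entry until it completes.
; Separate start and stop events set and clear a non-looping, zero-time timer bound to FireProjectile, which spawns BP_FireProjectile at ProjectileSpawnLocation.
; Tick stores movement speed in MoveSpeed.
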(event `self.ReceiveBeginPlay`
  (bind _asbp_character (cast `/Game/MyContent/BP_Character` (`GameplayStatics.GetPlayerCharacter` 0)))
  (set `self.As BP Character` _asbp_character))

(event `self.ReceiveTick`
  (params (DeltaSeconds :type "Float (single-precision)"))
  (set `self.MoveSpeed` (`KismetMathLibrary.VSize` (`MovementComponent.Velocity` (`self.CharacterMovement`)))))

(event `/Game/MyContent/Enemies/BossEnemy/BPI_BossFIght.Attack`
  (if (and (not (`self.isAttacking`)) (not (`/Game/MyContent/BP_Character.isDead` (`self.As BP Character`))))
    (`|PlayMontage` (`self.Mesh`) "/Game/MyContent/Enemies/BossEnemy/infinian-lineage-series/source/Infinian/Boss_RangedAttack.Boss_RangedAttack"
      (:`then`
        (set `self.isAttacking` true))
      (:`OnCompleted`
        (set `self.isAttacking` false)))))

(event `Start Fire Projectile`
  (bind _returnvalue (`KismetSystemLibrary.K2_SetTimerDelegate` (delegate `Fire Projectile`)))
  (set `self.ProjectileTimerHandle` _returnvalue))

(event `Fire Projectile`
  (`|SpawnActorFromClass` "/Game/MyContent/Enemies/BossEnemy/BP_FireProjectile.BP_FireProjectile_C" (`SceneComponent.K2_GetComponentToWorld` (`self.ProjectileSpawnLocation`)) "Undefined" "MultiplyWithRoot" null null))

(event `Stop Fire Projectile`
  (`KismetSystemLibrary.K2_ClearAndInvalidateTimerHandle` (`self.ProjectileTimerHandle`)))

(fn `UserConstructionScript`)