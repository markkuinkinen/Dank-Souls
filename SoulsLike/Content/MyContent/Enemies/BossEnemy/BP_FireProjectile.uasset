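; BP_FireProjectile is a boss enemy's gravity-free fire projectile that homes in on the player.
; On BeginPlay it sets BP_Character's capsule as the ProjectileMovement homing target.
; Hitting the player deals clamped damage, spawns an emitter, calls BossDamage and destroys itself, unless the player is dodging or blocking while strafing.
; Other hits or stopping also destroy it, and box collision hits broadcast OnProjectileImpact.
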(event `self.ReceiveBeginPlay`
  (bind _asbp_character (cast `/Game/MyContent/BP_Character` (`GameplayStatics.GetPlayerCharacter` 0)))
  (set `self.As BP Character` _asbp_character)
  (`self.Go To Target`))

(event `self.ReceiveHit`
  (params (MyComp :type "PrimitiveComponent Object Reference") (Other :type "Actor Object Reference") (OtherComp :type "PrimitiveComponent Object Reference") (bSelfMoved :type Boolean) (HitLocation :type "Vector Structure") (HitNormal :type "Vector Structure") (NormalImpulse :type "Vector Structure") (Hit :type "HitResult Structure (by ref)"))
  (bind _as_bp_character (`self.As BP Character`))
  (bind (_returnvalue_x _returnvalue_y _returnvalue_z) (`KismetMathLibrary.BreakVector` (`SceneComponent.K2_GetComponentLocation` (`Character.Mesh` (`self.Homing Target`)))))
  (if (== Other (`self.Homing Target`))
    (if (or (and (`/Game/MyContent/BP_Character.isBlocking` _as_bp_character) (`/Game/MyContent/BP_Character.Strafing` _as_bp_character)) (`/Game/MyContent/BP_Character.Dodging` _as_bp_character))
      (`KismetSystemLibrary.PrintString` "outskilled")
      (else
        (set `/Game/MyContent/BP_Character.Health` (`KismetMathLibrary.FClamp` (- (`/Game/MyContent/BP_Character.Health` _as_bp_character) 5.0) 0.0 100.0) _as_bp_character)
        (`self.K2_DestroyActor`)
        (`GameplayStatics.SpawnEmitterAtLocation` null (`KismetMathLibrary.MakeVector` _returnvalue_x _returnvalue_y (+ _returnvalue_z 75.0)))
        (`/Game/MyContent/BP_Character.BossDamage` (`self.As BP Character`))))
    (else
      (`self.K2_DestroyActor`))))

(event `Go To Target`
  (bind _projectilemovement (`self.ProjectileMovement`))
  ;[1 1 1] Sets player as homing target for enemy projectile
  (bind _homingtarget (`self.FindHomingTarget`))
  (set `ProjectileMovementComponent.HomingTargetComponent` _homingtarget _projectilemovement)
  (set `ProjectileMovementComponent.bIsHomingProjectile` true _projectilemovement))

(event `self.BoxCollision.OnComponentHit`
  (params (HitComponent :type "PrimitiveComponent Object Reference") (OtherActor :type "Actor Object Reference") (OtherComp :type "PrimitiveComponent Object Reference") (NormalImpulse :type "Vector Structure") (Hit :type "HitResult Structure (by ref)"))
  (`self.OnProjectileImpact` OtherActor Hit)
  (`KismetSystemLibrary.PrintString` "Hello"))

(event `self.ProjectileMovement.OnProjectileStop`
  (params (ImpactResult :type "HitResult Structure (by ref)"))
  (`self.K2_DestroyActor`))

(fn `FindHomingTarget`
  (returns (HomingTarget :type "SceneComponent Object Reference"))
  (bind _returnvalue (`GameplayStatics.GetActorOfClass` "/Game/MyContent/BP_Character.BP_Character_C"))
  (set `self.Homing Target` _returnvalue)
  (return (`Character.CapsuleComponent` (`self.Homing Target`))))

(fn `UserConstructionScript`
  (bind _speed (`self.Speed`))
  (bind _projectilemovement (`self.ProjectileMovement`))
  (set `ProjectileMovementComponent.InitialSpeed` _speed _projectilemovement)
  (set `ProjectileMovementComponent.MaxSpeed` _speed _projectilemovement)
  (set `ProjectileMovementComponent.ProjectileGravityScale` 0.0 _projectilemovement))