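; Enemy AI pawn that spots the player and makes melee sword attacks.
; Pawn sensing flags the player as seen on the AI controller's blackboard.
; AttackPlayer sphere-traces ahead for the third-person character, plays the attack montage, then applies damage once it finishes.
; The construction script snaps the sword to the hand socket, and several disconnected leftover nodes never run.
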(event `self.PawnSensing.OnSeePawn`
  (params (Pawn :type "Pawn Object Reference"))
  ;[1 1 1] Detecting Player
  (cast `/Game/ThirdPerson/Blueprints/BP_ThirdPersonCharacter` Pawn)
  (`BlackboardComponent.SetValueAsBool` (`AIBlueprintHelperLibrary.GetBlackboard` (`AIBlueprintHelperLibrary.GetAIController` self)) "hasSeenPlayer" true))

(event `AttackPlayer`
  (bind _returnvalue (`self.K2_GetActorLocation`))
  ;[0.845 0.1633 1] attack
  (bind (_outhit _returnvalue_2) (`KismetSystemLibrary.SphereTraceSingleForObjects` :`Start` _returnvalue :`End` (+ _returnvalue (* (`KismetMathLibrary.GetForwardVector` (`self.K2_GetActorRotation`)) 250.0)) :`Radius` 120.0 :`ObjectTypes` (`|MakeArray` "ObjectTypeQuery3" :!type "EObjectTypeQuery Enum") :`bTraceComplex` true :`DrawDebugType` "ForDuration" :`TraceColor` (struct :`G` 0.814825 :`B` 1.0 :`A` 1.0) :`TraceHitColor` (struct :`R` 0.967913 :`G` 0.128666 :`B` 1.0 :`A` 1.0)))
  (if _returnvalue_2
    (bind (_bblockinghit _binitialoverlap _time _distance _location _impactpoint _normal _impactnormal _physmat _hitactor) (`GameplayStatics.BreakHitResult` _outhit))
    (cast `/Game/ThirdPerson/Blueprints/BP_ThirdPersonCharacter` _hitactor)
    (bind _returnvalue_3 (`self.PlayAnimMontage` "/Game/MyContent/Enemies/anims/Attack_MOntage.Attack_MOntage"))
    (`KismetSystemLibrary.Delay` _returnvalue_3)
    (`GameplayStatics.ApplyDamage` _hitactor 10.0)))

(event `CustomEvent`
  ;[0.845 0.1633 1] attack
)

(fn `UserConstructionScript`
  (`SceneComponent.K2_AttachToComponent` (`self.sword`) (`self.Mesh`) "hand_rSocket" "SnapToTarget" "SnapToTarget" "KeepRelative" true))