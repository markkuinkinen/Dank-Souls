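; Melee sword enemy that sits at its start point, chases and attacks the player when sensed or in range, and otherwise walks back.
; Tick drives the AI; overlap volumes gate chasing and attacks, while a looping timer line-traces between sword sockets to apply damage.
; Damage updates a health widget and plays impact or death montages, with hit reactions blocking further damage.
; Death ragdolls the mesh; the GameMode's player-spawn flag resets the enemy.
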(event `self.ReceiveBeginPlay`
  ;[1 0 0.07009] Begin
  ;[1 0.8475 0.2776] Staring location/anim
  (set `self.StartingPoint` (`self.K2_GetActorLocation`))
  (`self.PlayAnimMontage` "/Game/MyContent/Enemies/anims/sitting_enemy.sitting_enemy")
  ;[0.2977 1 0.3244] health widget
  (bind _asbp_character (cast `/Game/MyContent/BP_Character` (`GameplayStatics.GetPlayerCharacter` 0)))
  (set `self.As BP Character` _asbp_character)
  (bind _asai_health_widget (cast `/Game/MyContent/Enemies/MarkkuENEMY/AI_HealthWidget` (`WidgetComponent.GetUserWidgetObject` (`self.HealthWidget`))))
  (set `self.HealthWidgetRef` _asai_health_widget))

(event `self.ReceiveTick`
  (params (DeltaSeconds :type "Float (single-precision)"))
  (bind _mesh (`self.Mesh`))
  (bind _mesh_2 (`self.Mesh`))
  ;[1 0 0] Event tick
  (`|ExecutionSequence`
    (:`then_0`
      ;[0.3922 0.8392 1] follow player
      (`self.ShowHealth`)
      (if (or (`self.canSeePlayer`) (`self.playerInRange`))
        (`self.StopAnimMontage` "/Game/MyContent/Enemies/anims/sitting_enemy.sitting_enemy")
        (`self.FollowPlayer`)
        (elif (and (`self.canSeePlayer`) (`self.playerInRange`))
          (`self.FollowPlayer`)
          (else
            ;[1 0.9033 0.4158] Back to start pos
            (`|AIMoveTo` self (`self.StartingPoint`) null 15.0
              (:`OnSuccess`
                (`self.PlayAnimMontage` "/Game/MyContent/Enemies/anims/sitting_enemy.sitting_enemy")))))))
    (:`then_1`
      ;[0.1922 0 1] Check if Ragdol
      (if (`self.RagdollMode`)
        (`SceneComponent.K2_SetWorldLocation` (`self.CapsuleComponent`) (- (`SceneComponent.GetSocketLocation` (`self.Mesh`) "None") (0.0 0.0 83.76)) false false)))
    (:`then_2`
      ;[0.1922 0 1] SET Ragdoll Mode Death
      (if (not (`self.isAlive`))
        (`PrimitiveComponent.SetCollisionProfileName` _mesh "Ragdoll" true)
        (`PrimitiveComponent.SetSimulatePhysics` _mesh true)
        (set `self.RagdollMode` true)))
    (:`then_3`
      ;[0.9783 0.9366 1] Resest enemy when player dies
      (bind _asbp_game_mode (cast `/Game/MyContent/BP_GameMode` (`GameplayStatics.GetGameMode`)))
      (if (`/Game/MyContent/BP_GameMode.PlayerSpawned` _asbp_game_mode)
        (set `/Game/MyContent/BP_GameMode.PlayerSpawned` false _asbp_game_mode)
        (set `self.isAlive` true)
        (`self.K2_SetActorLocation` (`self.StartingPoint`))
        (set `self.currentHealth` (`self.MaxHealth`))
        ;[0.1922 0 1] Reset rgdoll
        (set `self.RagdollMode` false)
        (`PrimitiveComponent.SetSimulatePhysics` _mesh_2 false)
        (`PrimitiveComponent.SetCollisionProfileName` _mesh_2 "CharacterMesh" true)
        (`SceneComponent.K2_AttachToComponent` _mesh_2 (`self.CapsuleComponent`) "None" "KeepWorld" "KeepWorld" "KeepWorld" true)
        (`SceneComponent.K2_SetRelativeLocationAndRotation` _mesh_2 (0.0 0.0 -83.761096) (struct :`Yaw` -90.0) false false)))))

(event `self.PawnSensing.OnSeePawn`
  (params (Pawn :type "Pawn Object Reference"))
  ;[0.3922 0.8392 1] Follow Player
  (set `self.canSeePlayer` true))

(event `FollowPlayer`
  ;[0.3922 0.8392 1] Follow Player
  (bind _returnvalue (`self.ActorToCheck` (`GameplayStatics.GetPlayerCharacter` 0)))
  (if _returnvalue
    _
    (else
      _))
  (`self.Rotate`)
  (`|AIMoveTo` self (0.0 0.0 0.0) (`GameplayStatics.GetPlayerCharacter` 0) 70.0
    (:`OnSuccess`
      ;[1 0.03529 0.07059] Attack Player
      (if (and (`self.canAttack`) (`self.AbleToAttack`))
        (set `self.canAttack` false)
        (`MovementComponent.StopMovementImmediately` (`self.CharacterMovement`))
        (bind _returnvalue_2 (`self.PlayAnimMontage` "/Game/MyContent/Enemies/anims/Attack_MOntage.Attack_MOntage" 1.3))
        (`KismetSystemLibrary.Delay` (- _returnvalue_2 0.6))
        (set `self.canAttack` true)))))

(event `self.Box1.OnComponentBeginOverlap`
  (params (OverlappedComponent :type "PrimitiveComponent Object Reference") (OtherActor :type "Actor Object Reference") (OtherComp :type "PrimitiveComponent Object Reference") (OtherBodyIndex :type Integer) (bFromSweep :type Boolean) (SweepResult :type "HitResult Structure (by ref)"))
  ;[0.251 0.4078 0.3529] Rotate
  (cast `/Game/MyContent/BP_Character` OtherActor)
  (`self.Rotate`))

(event `TriggerSword`
  ;[1 0.03529 0.07059] Set sword collider (trigger) active/inactive, apply damage
  (bind _returnvalue (`KismetSystemLibrary.K2_SetTimerDelegate` (delegate `SwordLineTrace`) 0.01 true))
  (set `self.TriggerSwordEvent` _returnvalue))

(event `SwordLineTrace`
  (bind _sword (`self.Sword`))
  ;[1 0.03529 0.07059] Set sword collider (trigger) active/inactive, apply damage
  (bind _outhit (`KismetSystemLibrary.LineTraceSingle` :`Start` (`SceneComponent.GetSocketLocation` _sword "start") :`End` (`SceneComponent.GetSocketLocation` _sword "end") :`TraceChannel` "TraceTypeQuery2" :`DrawDebugType` "ForDuration" :`DrawTime` 0.2))
  (bind (_bblockinghit _binitialoverlap _time _distance _location _impactpoint _normal _impactnormal _physmat _hitactor) (`GameplayStatics.BreakHitResult` _outhit))
  (`KismetSystemLibrary.PrintString` (`KismetSystemLibrary.GetDisplayName` _hitactor))
  (`GameplayStatics.ApplyDamage` _hitactor 50.0 (`self.GetController`) self))

(event `Rotate`
  (bind (_returnvalue_roll _returnvalue_pitch _returnvalue_yaw) (`KismetMathLibrary.BreakRotator` (`KismetMathLibrary.RInterpTo` (`self.K2_GetActorRotation`) (`KismetMathLibrary.FindLookAtRotation` (`self.K2_GetActorLocation`) (`self.K2_GetActorLocation` (`GameplayStatics.GetPlayerCharacter` 0))) (`GameplayStatics.GetWorldDeltaSeconds`) 1.0)))
  ;[0.251 0.4078 0.3529] facing the player if in rAange
  (if (`self.playerInRange`)
    (`self.K2_SetActorRotation` (`KismetMathLibrary.MakeRotator` 0.0 0.0 _returnvalue_yaw))))

(event `StopTriggerSword`
  ;[1 0.03529 0.07059] Set sword collider (trigger) active/inactive, apply damage
  (`KismetSystemLibrary.K2_ClearAndInvalidateTimerHandle` (`self.TriggerSwordEvent`)))

(event `self.ReceiveAnyDamage`
  (params (Damage :type "Float (single-precision)") (DamageType :type "DamageType Object Reference") (InstigatedBy :type "Controller Object Reference") (DamageCauser :type "Actor Object Reference"))
  (bind _currenthealth (`self.currentHealth`))
  ;[1 0.03439 0.7938] Taking damage and Death
  (`/Engine/EditorBlueprintResources/StandardMacros.DoOnce` false :!label _label
    (:`Completed`
      (if (>= (- _currenthealth Damage) 0.0)
        (bind _output_get (set `self.currentHealth` (- _currenthealth Damage)))
        (set `/Game/MyContent/Enemies/MarkkuENEMY/AI_HealthWidget.Health` _output_get (`self.HealthWidgetRef`))
        (if (<= (`self.currentHealth`) 0.0)
          (`MovementComponent.StopMovementImmediately` (`self.CharacterMovement`))
          (set `self.canAttack` false)
          (`self.PlayAnimMontage` "/Game/MyContent/Enemies/EnemyModel/enemy_death.enemy_death")
          (set `self.isAlive` false)
          (else
            (`MovementComponent.StopMovementImmediately` (`self.CharacterMovement`))
            (bind _returnvalue (`self.PlayAnimMontage` "/Game/MyContent/Enemies/EnemyModel/enemy_impact.enemy_impact"))
            (`KismetSystemLibrary.Delay` _returnvalue)
            (goto _label :!via `Reset`)))))))

(event `self.Sphere.OnComponentBeginOverlap`
  (params (OverlappedComponent :type "PrimitiveComponent Object Reference") (OtherActor :type "Actor Object Reference") (OtherComp :type "PrimitiveComponent Object Reference") (OtherBodyIndex :type Integer) (bFromSweep :type Boolean) (SweepResult :type "HitResult Structure (by ref)"))
  ;[0.2353 0.2784 0.4078] Toggle player in range (from distance)
  (cast `/Game/MyContent/BP_Character` OtherActor)
  (set `self.playerInRange` true))

(event `self.Box.OnComponentBeginOverlap`
  (params (OverlappedComponent :type "PrimitiveComponent Object Reference") (OtherActor :type "Actor Object Reference") (OtherComp :type "PrimitiveComponent Object Reference") (OtherBodyIndex :type Integer) (bFromSweep :type Boolean) (SweepResult :type "HitResult Structure (by ref)"))
  ;[0.2353 0.2784 0.4078] Comment
  (cast `/Game/MyContent/BP_Character` OtherActor)
  (set `self.AbleToAttack` true))

(event `self.Box.OnComponentEndOverlap`
  (params (OverlappedComponent :type "PrimitiveComponent Object Reference") (OtherActor :type "Actor Object Reference") (OtherComp :type "PrimitiveComponent Object Reference") (OtherBodyIndex :type Integer))
  ;[0.2353 0.2784 0.4078] Comment
  (cast `/Game/MyContent/BP_Character` OtherActor)
  (set `self.AbleToAttack` false))

(event `self.Sphere.OnComponentEndOverlap`
  (params (OverlappedComponent :type "PrimitiveComponent Object Reference") (OtherActor :type "Actor Object Reference") (OtherComp :type "PrimitiveComponent Object Reference") (OtherBodyIndex :type Integer))
  ;[0.2353 0.2784 0.4078] Toggle player in range (from distance)
  (cast `/Game/MyContent/BP_Character` OtherActor)
  (set `self.playerInRange` false))

(fn `ActorToCheck`
  (params (Actor :type "Actor Object Reference"))
  (returns (ReturnValue :type Boolean))
  (bind _capsulecomponent (`self.CapsuleComponent`))
  (return (< (`KismetMathLibrary.DegAcos` (`KismetMathLibrary.Dot_VectorVector` (`KismetMathLibrary.Vector_Normal2D` (- (`self.K2_GetActorLocation` Actor) (`SceneComponent.K2_GetComponentLocation` _capsulecomponent))) (`SceneComponent.GetForwardVector` _capsulecomponent))) 60.0)))

(fn `ShowHealth`
  (bind _healthwidget (`self.HealthWidget`))
  (if (and (< (`self.currentHealth`) (`self.MaxHealth`)) (> (`self.currentHealth`) 0.0) (`self.playerInRange`))
    (`SceneComponent.SetVisibility` _healthwidget true false)
    (set `self.canSeePlayer` true)
    (else
      (`SceneComponent.SetVisibility` _healthwidget false false)
      (set `self.canSeePlayer` false))))

(fn `UserConstructionScript`
  (`SceneComponent.K2_AttachToComponent` (`self.Sword`) (`self.Mesh`) "hand_rSocket" "KeepRelative" "KeepRelative" "KeepRelative" true))