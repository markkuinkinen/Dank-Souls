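; Enemy character Blueprint that roams, chases the player on sight and makes melee attacks, with a weapon attached to its hand socket.
; AIMoveTo roams to random reachable points until PawnSensing triggers a chase of the player character.
; On arrival, a debug-drawn sphere trace, ending at the raw forward vector rather than an offset, gates an attack montage and delayed damage.
; IsSeeingPlayer is never cleared, so the chase's roam fallback is effectively unreachable.
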(event `Random Roam`
  ;[1 1 1] ai roam
  (`|AIMoveTo` self (`NavigationSystemV1.K2_GetRandomReachablePointInRadius` (`self.K2_GetActorLocation`) 1000.0 null null) null
    (:`OnSuccess`
      (`self.Random Roam`))))

(event `self.ReceiveBeginPlay`
  (`self.Random Roam`))

(event `self.PawnSensing.OnSeePawn`
  (params (Pawn :type "Pawn Object Reference"))
  (set `self.isSeeingPlayer` true)
  (`self.Follow Player`))

(event `self.ReceiveTick`
  (params (DeltaSeconds :type "Float (single-precision)")))

(event `Follow Player`
  (set `self.canAttack` true)
  (if (`self.isSeeingPlayer`)
    (`|AIMoveTo` self (0.0 0.0 0.0) (`GameplayStatics.GetPlayerCharacter` 0) 70.0
      (:`OnSuccess`
        (if (`self.canAttack`)
          (bind (_outhit _returnvalue) (`KismetSystemLibrary.SphereTraceSingleForObjects` :`Start` (`self.K2_GetActorLocation`) :`End` (`KismetMathLibrary.GetForwardVector` (`self.K2_GetActorRotation`)) :`Radius` 120.0 :`ObjectTypes` (`|MakeArray` "ObjectTypeQuery3" :!type "EObjectTypeQuery Enum") :`DrawDebugType` "ForDuration" :`TraceColor` (struct :`G` 0.814825 :`B` 1.0 :`A` 1.0) :`TraceHitColor` (struct :`R` 0.967913 :`G` 0.128666 :`B` 1.0 :`A` 1.0)))
          (if _returnvalue
            (bind (_bblockinghit _binitialoverlap _time _distance _location _impactpoint _normal _impactnormal _physmat _hitactor) (`GameplayStatics.BreakHitResult` _outhit))
            (cast `/Game/ThirdPerson/Blueprints/BP_ThirdPersonCharacter` _hitactor
              (:`then`
                (bind _returnvalue_2 (`self.PlayAnimMontage` "/Game/MyContent/Enemies/anims/Attack_MOntage.Attack_MOntage"))
                (set `self.canAttack` false)
                (`KismetSystemLibrary.Delay` _returnvalue_2)
                (`GameplayStatics.ApplyDamage` _hitactor 10.0)
                (set `self.canAttack` true))
              (:`CastFailed`
                (`KismetSystemLibrary.PrintString` "Hello")))))))
    (else
      (set `self.isSeeingPlayer` true)
      (`KismetSystemLibrary.RetriggerableDelay` 1.0)
      (`self.Random Roam`))))

(fn `UserConstructionScript`
  (`SceneComponent.K2_AttachToComponent` (`self.weapon`) (`self.Mesh`) "hand_rSocket" "SnapToTarget" "SnapToTarget" "KeepRelative" true))